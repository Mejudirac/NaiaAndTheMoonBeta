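; BP_FollowCamera is a camera actor that follows the player's BP_MainCharacter from a fixed offset behind on world X and high above.
; Every Tick it sets itself as the player controller's view target, then teleports its SpringArm to the character's location plus that offset.
; The offset is in world space, so the camera position ignores the character's rotation.
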(event `self.ReceiveTick`
  (params (DeltaSeconds :type "Float (single-precision)"))
  (`PlayerController.SetViewTargetWithBlend` (`PlayerState.GetPlayerController` (`Pawn.PlayerState` (`GameplayStatics.GetPlayerPawn` 0))) self 0.0 "VTBlend_Linear" 0.0 false)
  (bind _asbp_main_character (cast `/Game/NaiaAndTheMoon/Characters/MainCharacter/BP_MainCharacter` (`GameplayStatics.GetPlayerCharacter` 0)))
  (bind (_returnvalue_x _returnvalue_y _returnvalue_z) (`KismetMathLibrary.BreakVector` (`self.K2_GetActorLocation` _asbp_main_character)))
  (`SceneComponent.K2_SetWorldLocation` (`self.SpringArm`) (`KismetMathLibrary.MakeVector` (- _returnvalue_x 500.0) (- _returnvalue_y 0.0) (+ _returnvalue_z 1000.0)) false true))

(fn `UserConstructionScript`)