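; BP_MeleeMonkey is a melee monkey enemy that chases the player and punches.
; Pawn sensing sets IsSeen and calls FollowPlayer, which moves the monkey to the player with AI MoveTo.
; On arrival it plays a punch montage, using CanAttack and a montage-length delay as a gate.
; Damage comes separately from capsule hits on any actor, throttled by a DoOnce that resets after a one-second delay.
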(event `self.ReceiveTick`
  (params (DeltaSeconds :type "Float (single-precision)"))
  (if (`self.IsSeen`)
    _))

(event `self.PawnSensing.OnSeePawn`
  (params (Pawn :type "Pawn Object Reference"))
  (set `self.IsSeen` true)
  (`self.Follow Player`))

(event `Follow Player`
  (set `self.CanAttack?` true)
  (if (`self.IsSeen`)
    (`|AIMoveTo` self (0.0 0.0 0.0) (`GameplayStatics.GetPlayerCharacter` 0)
      (:`OnSuccess`
        (if (`self.CanAttack?`)
          (set `self.CanAttack?` false)
          (bind _returnvalue (`self.PlayAnimMontage` "/Game/NaiaAndTheMoon/Characters/Animals/Monkey/Melee/Animation/AM_PunchMunkey_Montage.AM_PunchMunkey_Montage"))
          (`KismetSystemLibrary.Delay` _returnvalue)
          (set `self.CanAttack?` true))))
    (else
      (set `self.IsSeen` false))))

(event `self.CapsuleComponent.OnComponentHit`
  (params (HitComponent :type "PrimitiveComponent Object Reference") (OtherActor :type "Actor Object Reference") (OtherComp :type "PrimitiveComponent Object Reference") (NormalImpulse :type "Vector Structure") (Hit :type "HitResult Structure (by ref)"))
  (`/Engine/EditorBlueprintResources/StandardMacros.DoOnce` false :!label _label
    (:`Completed`
      (`GameplayStatics.ApplyDamage` OtherActor 33.333334 null self)
      (`KismetSystemLibrary.Delay` 1.0)
      (goto _label :!via `Reset`))))

(fn `UserConstructionScript`)