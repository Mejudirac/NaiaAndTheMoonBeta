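; Spike trap obstacle that raises its spike and damages an actor entering its Box trigger.
; On overlap, the Spike_ timeline lerps the spike from SpikeDown to SpikeUp, reversing one second after overlap ends.
; Timeline updates apply damage to the overlapping actor through a DoOnce that resets after a one-second delay.
; The construction script applies configurable meshes and a shared material to spike and base.
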(event `self.Box.OnComponentBeginOverlap`
  (params (OverlappedComponent :type "PrimitiveComponent Object Reference") (OtherActor :type "Actor Object Reference") (OtherComp :type "PrimitiveComponent Object Reference") (OtherBodyIndex :type Integer) (bFromSweep :type Boolean) (SweepResult :type "HitResult Structure (by ref)"))
  (bind (_direction _newtrack_0) (`Timeline|Spike_` :!label _label)
    (:`Update`
      (`SceneComponent.K2_SetRelativeLocation` (`self.Spike`) (`KismetMathLibrary.VLerp` (`KismetMathLibrary.MakeVector` 0.0 0.0 (`self.Spike Down`)) (`KismetMathLibrary.MakeVector` 0.0 0.0 (`self.Spike Up`)) _newtrack_0) false false)
      (`/Engine/EditorBlueprintResources/StandardMacros.DoOnce` false :!label _label_2
        (:`Completed`
          (`GameplayStatics.ApplyDamage` OtherActor 33.333334 null self)
          (`KismetSystemLibrary.Delay` 1.0)
          (goto _label_2 :!via `Reset`))))))

(event `self.Box.OnComponentEndOverlap`
  (params (OverlappedComponent :type "PrimitiveComponent Object Reference") (OtherActor :type "Actor Object Reference") (OtherComp :type "PrimitiveComponent Object Reference") (OtherBodyIndex :type Integer))
  (`KismetSystemLibrary.Delay` 1.0)
  (goto _label :!via `Reverse`))

(fn `UserConstructionScript`
  (`PrimitiveComponent.SetMaterial` (`self.Spike`) 0 (`self.Material`))
  (`PrimitiveComponent.SetMaterial` (`self.Base`) 0 (`self.Material`))
  (`StaticMeshComponent.SetStaticMesh` (`self.Spike`) (`self.Static Mesh Spike`))
  (`StaticMeshComponent.SetStaticMesh` (`self.Base`) (`self.Static Mesh Base`)))